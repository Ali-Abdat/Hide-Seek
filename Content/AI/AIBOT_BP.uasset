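; Hide-and-seek enemy bot that restarts the level if the player starts too close or gets caught.
; PawnSensing triggers a chase to the player's seen location, returning to spawn if already there.
; AIPerception stimuli draw it slowly to investigate, then a looping timer interpolates it to a random yaw.
; It then carries overlapping displaced SmallPickableCubes to their stored location before heading home.
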(event `self.ReceiveBeginPlay`
  ;[0.124 1 0] If the Bot Near the Player by 1000 Restart the Game
  (`self.K2_SetActorRotation` (`KismetMathLibrary.MakeRotator` 0.0 0.0 (`KismetMathLibrary.RandomFloatInRange` -180.0 180.0)))
  (`PawnSensingComponent.SetPeripheralVisionAngle` (`self.PawnSensing`) (/ (`self.FieldOfView`) 2.0))
  (`KismetSystemLibrary.Delay` 1.0)
  (set `self.SpawnLocation` (`self.K2_GetActorLocation`))
  (if (<= (`self.GetDistanceTo` (`GameplayStatics.GetPlayerPawn` 0) self) 1000.0)
    (`GameplayStatics.OpenLevel` "HideAndSeekMap")))

(event `self.ReceiveTick`
  (params (DeltaSeconds :type "Float (single-precision)"))
  (set `self.Delta Seconds` DeltaSeconds)
  ;[0.03384 1 0] When The Bot Becomes Near the Pawn within 150 Restart the level
  (if (<= (`self.GetDistanceTo` (`GameplayStatics.GetPlayerPawn` 0) self) 150.0)
    (`/Engine/EditorBlueprintResources/StandardMacros.DoOnce` false
      (:`Completed`
        (`GameplayStatics.OpenLevel` "HideAndSeekMap")))))

(event `self.PawnSensing.OnSeePawn`
  (params (Pawn :type "Pawn Object Reference"))
  ;[0.1258 1 0] Going towards the Characters when He Sees Him
  (bind _asfirst_person_character (cast `/Game/FirstPersonCPP/Blueprints/FirstPersonCharacter` Pawn))
  (bind _output_get (set `self.pawnPlayer` _asfirst_person_character))
  (`KismetSystemLibrary.K2_ClearAndInvalidateTimerHandle` (`self.LookAroundTimer`))
  (set `self.PawnDest` (`self.K2_GetActorLocation` _output_get))
  (set `self.SawTheEnemy` true)
  (set `CharacterMovementComponent.MaxWalkSpeed` (`self.ChasingSpeed`) (`self.CharacterMovement`) :!label _label)
  (bind _returnvalue (`AIController.MoveToLocation` (`AIBlueprintHelperLibrary.GetAIController` self) (`self.PawnDest`) -1.0 true true false true null true))
  ;[1 0 0.03065] Returning Back to the Spawn Point
  (switch `EPathFollowingRequestResult` _returnvalue
    (:`AlreadyAtGoal`
      (set `self.pawnPlayer` null)
      (set `self.SawTheEnemy` false)
      (`self.ReturnBackHome`))))

(event `self.AIPerception.OnTargetPerceptionUpdated`
  (params (Actor :type "Actor Object Reference") (Stimulus :type "AIStimulus Structure"))
  ;[0.06004 1 0] Going to the ThrownObject
  (cast `AIBot` Actor
    (:`CastFailed`
      (if (`self.SawTheEnemy`)
        (goto _label)
        (else
          (set `CharacterMovementComponent.MaxWalkSpeed` (* (`self.ChasingSpeed`) 0.2) (`self.CharacterMovement`))
          (`|AIMoveTo` self Stimulus_StimulusLocation null 100.0
            (:`OnSuccess`
              (`self.LookAroundRandomAngle`))))))))

(event `StartMoving`
  (bind _noise_object (`self.Noise_Object`))
  (bind _noise_object_2 (`self.Noise_Object`))
  ;[1 1 1] After Reaching to the noise point
  (for _array_element (`PrimitiveComponent.GetOverlappingActors` (`self.SphereComp`) "/Script/Engine.Actor")
    (bind _assmall_pickable_cubes (cast `SmallPickableCubes` _array_element))
    (if (`SmallPickableCubes.IsChangedLocation` _assmall_pickable_cubes)
      (bind _output_get (set `self.Noise_Object` _assmall_pickable_cubes))
      (set `self.Current Loc` (`SmallPickableCubes.CurrentLoc` _noise_object_2))
      (`PrimitiveComponent.SetSimulatePhysics` (`StaticMeshActor.StaticMeshComponent` _noise_object_2) false)
      (`self.K2_AttachToComponent` _output_get (`self.Pickingup_`) "None" "SnapToTarget" "KeepRelative" "KeepRelative" true)
      (`|AIMoveTo` self (`self.Current Loc`) null 250.0
        (:`OnSuccess`
          (`self.K2_DetachFromActor` _noise_object "KeepRelative" "KeepRelative" "KeepRelative")
          (`self.K2_SetActorLocation` _noise_object (`SmallPickableCubes.CurrentLoc` _noise_object) false false)
          (`self.ReturnBackHome`))))))

(event `self.SphereComp.OnComponentBeginOverlap`
  (params (OverlappedComponent :type "PrimitiveComponent Object Reference") (OtherActor :type "Actor Object Reference") (OtherComp :type "PrimitiveComponent Object Reference") (OtherBodyIndex :type Integer) (bFromSweep :type Boolean) (SweepResult :type "HitResult Structure (by ref)")))

(event `LookAroundRandomAngle`
  (bind (_returnvalue_roll _returnvalue_pitch _returnvalue_yaw) (`KismetMathLibrary.BreakRotator` (`KismetMathLibrary.RandomRotator` false)))
  ;[1 1 1] GetRandom Rotation and InterpSpeed for the Rotation
  (set `self.Interp Speed` (`KismetMathLibrary.RandomFloatInRange` 3.0 3.5))
  (set `self.Angle` _returnvalue_yaw)
  (bind _returnvalue (`KismetSystemLibrary.K2_SetTimer` null "IntervalRotation" 0.1 true))
  (set `self.LookAroundTimer` _returnvalue))

(fn `GettingArcSight`
  (returns (Arc :type "Float (double-precision)"))
  (return (`self.FieldOfView`)))

(fn `GettingRadiusSight`
  (returns (SightRadius :type "Float (double-precision)"))
  (return (`PawnSensingComponent.SightRadius` (`self.PawnSensing`))))

(fn `IntervalRotation`
  (locals (NewLocalVar_1 :type "Float (double-precision)" :default 0.0))
  (bind _angle (`self.Angle`))
  (bind _yaw (.yaw (`self.K2_GetActorRotation`)))
  (`self.K2_SetActorRotation` (`KismetMathLibrary.MakeRotator` 0.0 0.0 (`KismetMathLibrary.FInterpTo` _yaw _angle (`self.Delta Seconds`) (`self.Interp Speed`))))
  (if (`KismetMathLibrary.NearlyEqual_FloatFloat` (`KismetMathLibrary.SelectFloat` (- _angle 360.0) _angle (> _angle 180.0)) _yaw 10.0)
    (`KismetSystemLibrary.K2_ClearAndInvalidateTimerHandle` (`self.LookAroundTimer`))
    (`self.StartMoving`)))

(fn `ReturnBackHome`
  (set `CharacterMovementComponent.MaxWalkSpeed` (/ (`self.ChasingSpeed`) 2.0) (`self.CharacterMovement`))
  (`AIController.MoveToLocation` (`AIBlueprintHelperLibrary.GetAIController` self) (`self.SpawnLocation`) -1.0 true true false true null true))

(fn `UserConstructionScript`)